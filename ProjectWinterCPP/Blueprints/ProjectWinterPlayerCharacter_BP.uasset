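; Player character Blueprint that shows the default HUD and handles picking up health and coin pickups.
; On BeginPlay it creates the HUD widget and adds it to the player screen.
; Pressing E refreshes the reference to the level's first PickupCollection actor, then loops over its pickups for those near the player.
; Health pickups heal by their value, coins increment the score without using CoinValue, and both are destroyed.
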(event `self.ReceiveBeginPlay`
  ;[1 1 1] Confer the Default Player HUD upon the Player Character, when play begins for the PlayerCharacter
  (bind _returnvalue (`|CreateWidget` "/Game/ProjectWinterCPP/Blueprints/DefaultPlayerHUD_BP.DefaultPlayerHUD_BP_C"))
  (`UserWidget.AddToPlayerScreen` _returnvalue 0))

(event `Key|E`
  (params (Key :type "Key Structure" :default "AnyKey"))
  ;[1 1 1] Handle picking up Pickups
  (:`Pressed`
    (`self.Update Ref. To Pickup Collection`)
    (for _array_element (`PickupCollection.PrimaryCollectionComponent` (`self.LevelPickupCollectionRef`))
      (if (`Pickup.bIsPlayerNearPickup` _array_element)
        (switch `string` (`Pickup.PickupID` _array_element)
          (:`Health Pickup`
            (bind _ashealth_pickup (cast `HealthPickup` _array_element))
            (`self.ModifyHealth` (`HealthPickup.HealthValue` _ashealth_pickup) true)
            ;[1 1 1] Destroy the Pickup objects after the Player has picked them up
            (`self.K2_DestroyActor` _ashealth_pickup))
          (:`Coin Pickup`
            (bind _ascoin_pickup (cast `CoinPickup` _array_element))
            (`self.IncrementCurrentScore`)
            (`self.K2_DestroyActor` _ascoin_pickup)))))))

(fn `Update Ref. To Pickup Collection`
  ;[1 1 1] Update a reference pointer within the ProjectWinterPlayerCharacter class
  (bind _outactors (`GameplayStatics.GetAllActorsOfClass` null "/Script/GroupProjectTestBlue.PickupCollection"))
  (`self.UpdatePickupReferences` (`KismetArrayLibrary.Array_Get` _outactors)))

(fn `UserConstructionScript`)